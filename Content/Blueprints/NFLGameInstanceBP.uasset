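; NFL game instance that holds the data for the two teams in the current match.
; On Init it runs UpdateMatchData, which looks up TeamAName and TeamBName as rows in TeamAtlasDT and caches any rows found as TeamA and TeamB.
; GetMatchData returns both cached team entries to callers.
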(event Custom|UpdateMatchData
  (Utilities|FlowControl|Sequence
    (:then_0
      (bind _returnvalue (Utilities|GetDataTableRow "/Game/Blueprints/Data/TeamAtlasDT.TeamAtlasDT" (Variables|Default|GetTeamAName))
        (:then
          (Variables|MatchData|SetTeam%20A _returnvalue))))
    (:then_1
      (bind _returnvalue_2 (Utilities|GetDataTableRow "/Game/Blueprints/Data/TeamAtlasDT.TeamAtlasDT" (Variables|Default|GetTeamBName))
        (:then
          (Variables|MatchData|SetTeam%20B _returnvalue_2))))))

(event EventInit
  (CallFunction|UpdateMatchData))

(fn GetMatchData
  (return (Variables|MatchData|GetTeam%20A) (Variables|MatchData|GetTeam%20B)))