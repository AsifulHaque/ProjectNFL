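; Spectator pawn that either flies as a player-controlled free camera or auto-rotates on its own.
; An isFreeCam macro branches on the FreeCam flag to gate every axis input and the Tick logic.
; In free cam, movement follows the camera's forward and right vectors, while look input drives controller yaw and pitch.
; Otherwise Tick rotates the actor by a fixed step each frame, unscaled by delta time.
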(event EventTick
  (params (DeltaSeconds :type Float%20%28single-precision%29))
  ;[1 1 1] autorotate if not freeCam
  (Utilities|IsFreeCam
    (:false
      (Class|Actor|AddActorWorldRotation "0,0.200000, 0"))))

(event Input|AxisEvents|InputAxisMoveForward/Backwards
  (params (AxisValue :type Float%20%28single-precision%29))
  ;[1 1 1] Movement
  (Utilities|IsFreeCam
    (:true
      (Pawn|Input|AddMovementInput (Math|Vector|GetForwardVector (Variables|Default|GetCamera)) AxisValue false))))

(event Input|AxisEvents|InputAxisMoveRight/Left
  (params (AxisValue :type Float%20%28single-precision%29))
  ;[1 1 1] Movement
  (Utilities|IsFreeCam
    (:true
      (Pawn|Input|AddMovementInput (Math|Vector|GetRightVector (Variables|Default|GetCamera)) AxisValue false))))

(event Input|AxisEvents|InputAxisLookLeft/Right
  (params (AxisValue :type Float%20%28single-precision%29))
  ;[1 1 1] Look
  (Utilities|IsFreeCam
    (:true
      (Pawn|Input|AddControllerYawInput AxisValue))))

(event Input|AxisEvents|InputAxisLookUp/Down
  (params (AxisValue :type Float%20%28single-precision%29))
  ;[1 1 1] Look
  (Utilities|IsFreeCam
    (:true
      (Pawn|Input|AddControllerPitchInput AxisValue))))

(fn ConstructionScript)