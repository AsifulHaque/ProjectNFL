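; BallBP is a physics ball that characters can catch, hold and throw.
; A catch request through an interface disables physics and collision, snaps the ball to a socket on the character's mesh and sets that character's ball reference.
; Detach and throw clear the holder, restore physics and collision and make the ball catchable again.
; Throw also sets the launch velocity.
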(event Custom|AllowCharacterToCatch
  (params (PlayerCharacter :type Character%20Object%20Reference) (SocketName :type Name))
  (bind _ballmesh (Variables|Default|GetBallMesh))
  ;[1 0.3802 0] Server_Multicast
  (Variables|STATUS|SetCurrentHolder PlayerCharacter)
  (Physics|SetSimulatePhysics _ballmesh false)
  (Collision|SetCollisionEnabled _ballmesh "NoCollision")
  (bind _mesh (Class|BallInteractionInterfaceBP|GetCharMesh(Message) PlayerCharacter))
  (Transformation|AttachComponentToComponent _mesh SocketName "SnapToTarget" "SnapToTarget" "KeepWorld" true)
  (Class|BallInteractionInterfaceBP|SetCharBallRefonCatch(Message) PlayerCharacter self)
  (Variables|STATUS|SetIs%20Catchable? false))

(event EventThrow
  (params (LaunchVelocity :type Vector :default "0, 0, 0"))
  (bind _ballmesh (Variables|Default|GetBallMesh))
  ;[1 1 1] Detach
  (Class|BallInteractionInterfaceBP|SetCharBallRefonCatch(Message) (Variables|STATUS|GetCurrentHolder))
  (Transformation|DetachFromActor "KeepWorld" "KeepWorld" "KeepWorld")
  (Variables|STATUS|SetCurrentHolder 0)
  (Variables|STATUS|SetIs%20Catchable? true)
  (Collision|SetCollisionEnabled _ballmesh "QueryAndPhysics")
  (Physics|SetSimulatePhysics _ballmesh true)
  (Class|PrimitiveComponent|SetAllPhysicsLinearVelocity (Variables|Default|GetBallMesh) LaunchVelocity false))

(event EventPlayertoBallCatchRequest
  (params (PlayerChar :type Character%20Object%20Reference) (SocketName :type Name :default "None"))
  ;[0.5251 1 0] Interface Implementation
  (CallFunction|AllowCharactertoCatch PlayerChar SocketName))

(event EventDetachBall
  (bind _ballmesh (Variables|Default|GetBallMesh))
  ;[1 0.09896 0.09896] Detach
  (Class|BallInteractionInterfaceBP|SetCharBallRefonCatch(Message) (Variables|STATUS|GetCurrentHolder))
  (Transformation|DetachFromActor "KeepWorld" "KeepWorld" "KeepWorld")
  (Variables|STATUS|SetCurrentHolder 0)
  (Variables|STATUS|SetIs%20Catchable? true)
  (Collision|SetCollisionEnabled _ballmesh "QueryAndPhysics")
  (Physics|SetSimulatePhysics _ballmesh true))

(fn ConstructionScript)

(fn CharHasBall?
  (return false))

(fn GetCharMesh
  (return 0))

(fn IsCatchable
  (return (Variables|STATUS|GetIs%20Catchable?)))