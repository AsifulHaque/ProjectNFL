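; Team formation marker actor that spawns a team's starting offense or defense players at preset positions.
; On BeginPlay, only the authority requests the spawn, which looks up the team's row in the team atlas table by name.
; Each starter in the chosen lineup is resolved in the player atlas table and spawned as a MasterCharacterBP with that data.
; The actor's static mesh components serve as spawn markers, matched to players by array index.
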(event Custom|SERVER_ReqSpawnPlayer
  ;[1 1 1] Implement Spawn Player on Server
  (bind _returnvalue (Utilities|GetDataTableRow "/Game/Blueprints/Data/TeamAtlasDT.TeamAtlasDT" (Variables|TeamInfo|GetTeamName))
    (:then
      (CallFunction|SpawnPlayer _returnvalue))))

(event EventBeginPlay
  ;[1 1 1] Only Server Tries to Spawn player
  (Networking|SwitchHasAuthority
    (:Authority
      (CallFunction|SERVERReqSpawnPlayer))))

(fn ConstructionScript)

(fn SpawnPlayer
  (params (TeamDataStruct :type Team%20Data%20Struct%20Structure%20%28by%20ref%29))
  (bind (_teamname _logo _players _startingoffense _startingdefense) (Utilities|Struct|BreakTeamDataStruct TeamDataStruct))
  (bind _values (Utilities|Map|Values _startingoffense))
  (bind _values_2 (Utilities|Map|Values _startingdefense))
  (bind (_array_element _array_index) (Utilities|Array|ForEachLoopwithBreak (select (Variables|TeamInfo|GetOffenseTeam?) _values _values_2))
    (:LoopBody
      (bind _returnvalue (Utilities|GetDataTableRow "/Game/Blueprints/Data/PlayerAtlasDT.PlayerAtlasDT" (.RowName (Utilities|Struct|BreakDataTableRowHandle _array_element)))
        (:then
          (Game|SpawnActorfromClass "/Game/Blueprints/MasterCharacterBP.MasterCharacterBP_C" (Math|Transform|MakeTransform (.Location (Math|Transform|BreakTransform (Transformation|GetWorldTransform (Utilities|Array|Get(acopy) (Actor|GetComponentsByClass "/Script/Engine.StaticMeshComponent") _array_index)))) (.Rotation (Math|Transform|BreakTransform (Transformation|GetWorldTransform (Utilities|Array|Get(acopy) (Actor|GetComponentsByClass "/Script/Engine.StaticMeshComponent") _array_index))))) "Undefined" 0 _returnvalue 0))
        (:RowNotFound
          (Development|PrintString "PLAYER SPAWN FAILED!!!"))))))