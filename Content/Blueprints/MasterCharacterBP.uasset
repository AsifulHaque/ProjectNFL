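; Master character for a ball-passing game that catches, holds and throws a ball, with movement input along world axes.
; On authority, overlapping a catchable actor requests a catch at the right-hand socket; receiving the ball blends the view and possesses this character.
; Left click flashes index labels on nearby ALS characters' widgets, then lobs the ball at the first one using a suggested projectile velocity, communicating through interface messages.
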(event EventTick
  (params (DeltaSeconds :type Float%20%28single-precision%29))
  (|CallParentFunction DeltaSeconds))

(event Collision|EventActorBeginOverlap
  (params (OtherActor :type Actor%20Object%20Reference))
  (Networking|SwitchHasAuthority
    (:Authority
      (bind _iscatchable_ (Class|BallInteractionInterfaceBP|IsCatchable(Message) OtherActor))
      (if _iscatchable_
        (Class|BallInteractionInterfaceBP|PlayertoBallCatchRequest(Message) OtherActor self "Ball_R")))))

(event EventCheckPassablePlayers
  (params (passkey :type Integer))
  (bind _widget (Variables|Default|GetWidget))
  (Rendering|SetVisibility _widget true false)
  (bind _aspassme_w (Utilities|Casting|CastTopassmeW (UserInterface|GetWidget _widget)))
  (Rendering|Components|TextRender|SetText (Variables|/Game/Widgets/passmeW.passmeW_C|GetpassKeyText _aspassme_w) (Utilities|Text|ToText(Integer) passkey))
  (Utilities|FlowControl|Delay 3.0)
  (Rendering|SetVisibility (Variables|Default|GetWidget) false false))

(event EventSetCharBallRefonCatch
  (params (Ball :type Actor%20Object%20Reference))
  (bind _returnvalue (Game|GetPlayerController 0))
  (bind _self self)
  ;[1 1 1] OnCatch
  (bind _output_get (Variables|STATUS|SetBallRef Ball))
  (bind _output_get_2 (Variables|STATUS|SetHas%20Ball (Utilities|IsValid _output_get)))
  (if _output_get_2
    (Game|Player|SetViewTargetwithBlend _returnvalue _self 1.0 "VTBlend_Linear" 0.0 true)
    (Pawn|Possess _returnvalue _self)))

(event Input|AxisEvents|InputAxisMoveForward/Backwards
  (params (AxisValue :type Float%20%28single-precision%29))
  ;[1 1 1] Movement override
  (Pawn|Input|AddMovementInput "1.000000, 0, 0" AxisValue false))

(event Input|AxisEvents|InputAxisMoveRight/Left
  (params (AxisValue :type Float%20%28single-precision%29))
  ;[1 1 1] Movement override
  (Pawn|Input|AddMovementInput "0,1.000000, 0" AxisValue false))

(event Input|MouseEvents|LeftMouseButton
  (params (Key :type Key%20Structure :default "None"))
  (:Pressed
    (if (Variables|STATUS|GetHas%20Ball)
      (bind _outactors (Collision|SphereOverlapActors (Transformation|GetActorLocation) 5e+02 (Utilities|Array|MakeArray "ObjectTypeQuery3") "/ALSV4_CPP/AdvancedLocomotionV4/Blueprints/CharacterLogic/ALS_CharacterBP.ALS_CharacterBP_C" (Utilities|Array|MakeArray self)))
      (for (_array_element _array_index) _outactors
        (Class|BallInteractionInterfaceBP|CheckPassablePlayers(Message) _array_element _array_index))
      (CallFunction|PassBall 1e+03 (Utilities|Array|Get(acopy) _outactors)))))

(fn ConstructionScript
  (|CallParentFunction))

(fn PassBall
  (params (LaunchSpeed :type Float%20%28single-precision%29) (Target :type Actor%20Object%20Reference))
  (bind _ballref (Variables|STATUS|GetBallRef))
  (Utilities|IsValid Target
    (:Is%20Valid
      (bind _tossvelocity (Class|GameplayStatics|BlueprintSuggestProjectileVelocity (Transformation|GetActorLocation _ballref) (+ (Transformation|GetActorLocation Target) "0, 0,100.000000") LaunchSpeed 0.0 "DoNotTrace" 1e+01 false true))
      (Class|BallInteractionInterfaceBP|Throw(Message) _ballref _tossvelocity))
    (:Is%20Not%20Valid
      (Development|PrintString "Throw target not set"))))

(fn CharHasBall?
  (return (Variables|STATUS|GetHas%20Ball)))

(fn GetCharMesh
  (return (Variables|Character|GetMesh)))

(fn IsCatchable
  (return false))